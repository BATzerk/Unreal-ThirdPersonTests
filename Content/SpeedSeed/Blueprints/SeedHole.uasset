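; SeedHole is a color-keyed planting spot that accepts a seed, counts down until the flower ripens, then can be reaped.
; ColorID pulls ripen time, material and light color from MyGameInstance.
; Inventory changes, player overlap and state drive the highlight lights and particles, with timelines animating the ripe arrow and glow.
; A Delay on Tick paces the one-second countdown; ReapFlower hides the hole and notifies GameController_Blueprint.
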(event Custom|Heard_OnPlayerInventoryChanged
  ;[1 1 1] Bind Events
  (CallFunction|OnPlayerInventoryChanged))

(event EventTick
  (params (DeltaSeconds :type Float%20%28single-precision%29))
  (CallFunction|MakeTextFaceCamera)
  (Utilities|FlowControl|Delay 1.0)
  (if (Variables|Default|GetHasSeed)
    (Variables|Default|SetTimeUntilRipe (- (Variables|Default|GetTimeUntilRipe) 1.0))
    (CallFunction|UpdateCountdownText)
    (if (<= (Variables|Default|GetTimeUntilRipe) 0.0)
      (CallFunction|OnBecomeRipe))))

(event EventBeginPlay
  (CallFunction|InitProperties)
  (bind _asfarmer_character (Utilities|Casting|CastToFarmerCharacter (Game|GetPlayerCharacter 0)))
  (Variables|Default|SetFarmerCharacterRef _asfarmer_character)
  ;[1 1 1] Bind Events
  (EventDispatchers|BindEventtoOnPlayerInventoryChanged (Variables|/Game/SpeedSeed/Blueprints/FarmerCharacter.FarmerCharacter_C|GetInventoryComponent (Variables|Default|GetFarmerCharacterRef)) (delegate Custom|Heard_OnPlayerInventoryChanged))
  ;[1 1 1] Init Visuals
  (Rendering|SetVisibility (Variables|Default|GetGrowingGroup) false true)
  (Components|Activation|Deactivate (Variables|Default|GetPS_Ripened))
  ;[1 1 1] Ongoing Animations
  (Utilities|FlowControl|Sequence
    (:then_0
      (bind _arrowpos (Timeline|BounceCalloutArrow Play)
        (:Update
          (Transformation|SetRelativeLocation (Variables|Default|GetRipeArrow) _arrowpos false false))))
    (:then_1
      (bind _intensity (Timeline|OscillateMayInteractIntensity Play)
        (:Update
          (Rendering|Components|Light|SetIntensity (Variables|Default|GetL_MayInteract) _intensity))))))

(event Collision|EventActorBeginOverlap
  (params (OtherActor :type Actor%20Object%20Reference))
  ;[1 1 1] Overlap Events
  (Utilities|Casting|CastToFarmerCharacter OtherActor)
  (Variables|Default|SetIsPlayerTouchingMe true)
  (CallFunction|UpdateHighlights))

(event Collision|EventActorEndOverlap
  (params (OtherActor :type Actor%20Object%20Reference))
  ;[1 1 1] Overlap Events
  (Utilities|Casting|CastToFarmerCharacter OtherActor)
  (Variables|Default|SetIsPlayerTouchingMe false)
  (CallFunction|UpdateHighlights))

(fn ConstructionScript)

(fn InitProperties
  (bind _asmy_game_instance (Utilities|Casting|CastToMyGameInstance (Game|GetGameInstance)))
  (bind _return (Default|GetRipenDuration _asmy_game_instance (Variables|Default|GetColorID)))
  (Variables|Default|SetTimeUntilRipe _return)
  (bind _return_2 (Default|GetSeedMaterial _asmy_game_instance (Variables|Default|GetColorID)))
  (Rendering|Material|SetMaterial (Variables|Default|GetCylinderGrowing) 0 _return_2)
  (bind _asmy_game_instance_2 (Utilities|Casting|CastToMyGameInstance (Game|GetGameInstance)))
  (bind _return_3 (Default|GetSeedColor _asmy_game_instance_2 (Variables|Default|GetColorID)))
  (Rendering|Components|Light|SetLightColor (Variables|Default|GetL_MayInteract) (Math|Conversions|ToLinearColor(Color) _return_3) true))

(fn AcceptSeed
  (Variables|Default|SetHasSeed true)
  (Variables|Default|SetCanAcceptSeed false)
  (Rendering|SetVisibility (Variables|Default|GetGrowingGroup) true true)
  (CallFunction|UpdateCountdownText)
  (CallFunction|UpdateHighlights))

(fn OnBecomeRipe
  (Variables|Default|SetIsRipe true)
  (Rendering|SetVisibility (Variables|Default|Gett_TimeLeft) false true)
  (Rendering|SetVisibility (Variables|Default|GetRipeArrow) true true)
  (CallFunction|UpdateHighlights)
  (Components|Activation|Activate (Variables|Default|GetPS_Ripened) false))

(fn UpdateCountdownText
  (Rendering|Components|TextRender|SetText (Variables|Default|Gett_TimeLeft) (Utilities|Text|ToText(Integer) (Math|Float|Ceil (Variables|Default|GetTimeUntilRipe)))))

(fn UpdateHighlights
  (LocalVariables|SetMayInteract (or (Variables|Default|GetIsRipe) (Math|Boolean|ANDBoolean (Variables|Default|GetCanAcceptSeed) (Variables|Default|GetDoesPlayerHaveSeedForMe) (not (Variables|Default|GetWasReaped)))))
  (Rendering|SetVisibility (Variables|Default|GetL_MayInteract) (LocalVariables|GetMayInteract) false)
  (Rendering|SetVisibility (Variables|Default|GetL_WillInteract) (and (LocalVariables|GetMayInteract) (Variables|Default|GetIsPlayerTouchingMe)) true)
  (Components|Activation|SetActive (Variables|Default|GetPS_ReadyForSeed) (and (Variables|Default|GetCanAcceptSeed) (Variables|Default|GetDoesPlayerHaveSeedForMe)) false))

(fn MakeTextFaceCamera
  (Transformation|SetWorldRotation (Variables|Default|Gett_TimeLeft) (.Rotation (Math|Transform|BreakTransform (Transformation|GetActorTransform (Game|GetPlayerController 0)))) false false))

(fn ReapFlower
  (Variables|Default|SetWasReaped true)
  (Variables|Default|SetCanAcceptSeed false)
  (Variables|Default|SetHasSeed false)
  (CallFunction|UpdateHighlights)
  (Rendering|SetVisibility (Variables|Default|GetComponents) false true)
  (Collision|SetActorEnableCollision false)
  (Components|Activation|Activate (Variables|Default|GetPS_ReapedFlower) false)
  (bind _returnvalue (Actor|GetActorOfClass "/Game/SpeedSeed/Blueprints/GameController_Blueprint.GameController_Blueprint_C"))
  (bind _asgame_controller_blueprint (Utilities|Casting|CastToGameController_Blueprint _returnvalue)
    (:then
      (Default|OnFlowerReaped _asgame_controller_blueprint))
    (:CastFailed
      (Development|PrintString "ERROR! Scene needs a GameController_Blueprint!" true true "(R=1.000000,G=0.016369,B=0.000000,A=1.000000)" 5.0))))

(fn OnPlayerInventoryChanged
  (bind _return (Default|DoesInventoryContainSeed (Variables|Default|GetFarmerCharacterRef) (Variables|Default|GetColorID)))
  (Variables|Default|SetDoesPlayerHaveSeedForMe _return)
  (CallFunction|UpdateHighlights))