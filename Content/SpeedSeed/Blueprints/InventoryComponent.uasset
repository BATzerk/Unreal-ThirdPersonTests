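; InventoryComponent stores the seeds held by its owner in SpeedSeed and provides functions to add, remove and look them up.
; On BeginPlay it creates an InventoryWindow widget bound to itself on the player controller's HUD canvas, then empties the MySeeds array.
; Lookups search MySeeds linearly by ColorID, which also serves to find the seed matching a given seed hole.
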(event EventBeginPlay
  (CallFunction|InitHUD)
  (CallFunction|InitInventory))

(fn InitInventory
  (Utilities|Array|Resize (Variables|Default|GetMySeeds) 0))

(fn InitHUD
  (bind _returnvalue (UserInterface|CreateWidget "/Game/SpeedSeed/Blueprints/InventoryWindow.InventoryWindow_C" 0 self))
  (Variables|Default|SetInventoryWindow _returnvalue)
  (bind _asmy_player_controller (Utilities|Casting|CastToMyPlayerController (Game|GetPlayerController 0)))
  (bind _returnvalue_2 (Class|CanvasPanel|AddChildtoCanvas (Variables|/Game/SpeedSeed/Blueprints/HUD.HUD_C|GetHudCanvas (Variables|/Game/SpeedSeed/Blueprints/MyPlayerController.MyPlayerController_C|GetHudWidget _asmy_player_controller)) (Variables|Default|GetInventoryWindow)))
  (Class|CanvasPanelSlot|SetAutoSize _returnvalue_2 true)
  (Class|CanvasPanelSlot|SetAlignment _returnvalue_2 "(X=0.500000,Y=0.000000)")
  (Class|CanvasPanelSlot|SetAnchors _returnvalue_2 (Variables|Default|GetAnchors)))

(fn ContainsSeed
  (params (ColorID :type Integer))
  (bind _return (CallFunction|GetSeedbyColorID ColorID))
  (return (!= _return 0)))

(fn AddSeed
  (params (Seed :type Seed%20Object%20Reference))
  (Utilities|Array|Add (Variables|Default|GetMySeeds) Seed))

(fn GetSeedforHole
  (params (SeedHole :type Seed%20Hole%20Object%20Reference))
  (bind _return (CallFunction|GetSeedbyColorID (Variables|/Game/SpeedSeed/Blueprints/SeedHole.SeedHole_C|GetColorID SeedHole)))
  (return _return))

(fn GetSeedbyColorID
  (params (ColorID :type Integer))
  (bind _array_element (Utilities|Array|ForEachLoopwithBreak (Variables|Default|GetMySeeds))
    (:LoopBody
      (if (== ColorID (Variables|/Game/SpeedSeed/Blueprints/Seed.Seed_C|GetColorID _array_element))
        (return _array_element)))
    (:Completed
      (return 0))))

(fn RemoveSeed
  (params (Seed :type Seed%20Object%20Reference))
  (Utilities|Array|RemoveItem (Variables|Default|GetMySeeds) Seed))