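; GameController for SpeedSeed that checks whether the level is complete whenever its OnFlowerReaped function is called.
; It scans every SeedHole actor and fails on the first one not marked WasReaped, otherwise printing a green level-complete message on screen.
; A debug "level NOT complete yet." print sits on the all-reaped path, so it appears alongside the success message.
; BeginPlay is empty.
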(event EventBeginPlay)

(fn ConstructionScript)

(fn OnFlowerReaped
  (CallFunction|CheckifLevelComplete))

(fn CheckifLevelComplete
  (bind _return (CallFunction|AreAllFlowersReaped))
  (if _return
    (Development|PrintString "LEVEL COMPLETE!" true true "(R=0.000000,G=1.000000,B=0.051281,A=1.000000)" 1e+01)))

(fn AreAllFlowersReaped
  (bind _outactors (Actor|GetAllActorsOfClass "/Game/SpeedSeed/Blueprints/SeedHole.SeedHole_C"))
  (for _array_element _outactors
    (if (not (Variables|/Game/SpeedSeed/Blueprints/SeedHole.SeedHole_C|GetWasReaped _array_element))
      (return false)))
  (Development|PrintString "level NOT complete yet.")
  (return true))