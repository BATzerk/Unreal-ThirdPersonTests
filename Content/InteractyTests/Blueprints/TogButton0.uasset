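; TogButton0 is an interactable toggle button that switches a list of linked objects on or off.
; Hovering shows or hides a callout arrow, and interacting flips IsOn through SetIsOn, which also applies the initial state at BeginPlay.
; SetIsOn swaps the button body's on/off material and forwards the state to each entry in MyOnOffables via BI_OnOffable, stopping at the first failed cast.
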(event EventBeginPlay
  (CallFunction|SetIson (Variables|Default|GetIsOn)))

(event EventBeginHover
  (Development|SetHiddeninGame (Variables|Default|GetCalloutArrow) false false))

(event EventEndHover
  (Development|SetHiddeninGame (Variables|Default|GetCalloutArrow) true false))

(event EventBeginInteract
  (CallFunction|ToggleIson))

(fn ConstructionScript)

(fn SetIson
  (params (Val :type Boolean))
  (Variables|Default|SetIsOn Val)
  (CallFunction|UpdateButtonMaterial)
  (for _array_element (Variables|Default|GetMyOnOffables)
    (bind _asbi_on_offable (Utilities|Casting|CastToBI_OnOffable _array_element))
    (Default|SetIson _asbi_on_offable (Variables|Default|GetIsOn))))

(fn ToggleIson
  (CallFunction|SetIson (not (Variables|Default|GetIsOn))))

(fn UpdateButtonMaterial
  (if (Variables|Default|GetIsOn)
    (Rendering|Material|SetMaterial (Variables|Default|GetButtonBody) 0 "/Game/Materials/M_ButtonOn.M_ButtonOn")
    (else
      (Rendering|Material|SetMaterial (Variables|Default|GetButtonBody) 0 "/Game/Materials/M_ButtonOff.M_ButtonOff"))))