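; A floor button actor that turns on while something overlaps its trigger and drives linked on/off objects.
; On begin play and on each overlap begin or end, it recomputes its state from the trigger's overlapping component count, using a hack threshold to discount its own components.
; SetIsOn swaps the button material and forwards the state to MyOnOffables through the BI_OnOffable interface.
; The Interact event is empty.
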(event EventBeginPlay
  (CallFunction|UpdateIsonfromTrigger))

(event EventInteract
  (params (Character :type Character%20Object%20Reference)))

(event Collision|EventActorBeginOverlap
  (params (OtherActor :type Actor%20Object%20Reference))
  (CallFunction|UpdateIsonfromTrigger))

(event Collision|EventActorEndOverlap
  (params (OtherActor :type Actor%20Object%20Reference))
  (CallFunction|UpdateIsonfromTrigger))

(fn ConstructionScript)

(fn SetIson
  (params (Val :type Boolean))
  (Variables|Default|SetIsOn Val)
  (CallFunction|UpdateButtonMaterial)
  (for _array_element (Variables|Default|GetMyOnOffables)
    (bind _asbi_on_offable (Utilities|Casting|CastToBI_OnOffable _array_element))
    (Default|SetIson _asbi_on_offable (Variables|Default|GetIsOn))))

(fn UpdateButtonMaterial
  (if (Variables|Default|GetIsOn)
    (Rendering|Material|SetMaterial (Variables|Default|GetButtonBody) 0 "/Game/Materials/M_ButtonOn.M_ButtonOn")
    (else
      (Rendering|Material|SetMaterial (Variables|Default|GetButtonBody) 0 "/Game/Materials/M_ButtonOff.M_ButtonOff"))))

(fn UpdateIsonfromTrigger
  (CallFunction|SetIson (> (Utilities|Array|Length (Class|PrimitiveComponent|GetOverlappingComponents (Variables|Default|GetTrigger))) 1)))