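; Interactable toggle lever that switches a list of linked on/off objects in the InteractyTests area.
; Interact flips IsOn through SetIsOn, which also runs on BeginPlay to apply the initial state.
; SetIsOn snaps LeverBox to its on or off position, swaps its material, then passes the state to each MyOnOffables entry via BI_OnOffable.
; An AnimateLeverToPos timeline exists but is never triggered.
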(event EventBeginPlay
  (CallFunction|SetIson (Variables|Default|GetIsOn)))

(event EventInteract
  (params (Character :type Character%20Object%20Reference))
  (CallFunction|ToggleIson))

(fn ConstructionScript)

(fn SetIson
  (params (Val :type Boolean))
  (Variables|Default|SetIsOn Val)
  ;[1 1 1] Update my visuals
  (CallFunction|UpdateLeverPos)
  (CallFunction|UpdateButtonMaterial)
  ;[1 1 1] Tell my OnOffables
  (for _array_element (Variables|Default|GetMyOnOffables)
    (bind _asbi_on_offable (Utilities|Casting|CastToBI_OnOffable _array_element))
    (Default|SetIson _asbi_on_offable (Variables|Default|GetIsOn))))

(fn ToggleIson
  (CallFunction|SetIson (not (Variables|Default|GetIsOn))))

(fn UpdateButtonMaterial
  (if (Variables|Default|GetIsOn)
    (Rendering|Material|SetMaterial (Variables|Default|GetLeverBox) 0 "/Game/Materials/M_ButtonOn.M_ButtonOn")
    (else
      (Rendering|Material|SetMaterial (Variables|Default|GetLeverBox) 0 "/Game/Materials/M_ButtonOff.M_ButtonOff"))))

(fn UpdateLeverPos
  (if (Variables|Default|GetIsOn)
    (Transformation|SetRelativeLocation (Variables|Default|GetLeverBox) (Variables|Default|GetLeverPosOn) false false)
    (else
      (Transformation|SetRelativeLocation (Variables|Default|GetLeverBox) (Variables|Default|GetLeverPosOff) false false))))