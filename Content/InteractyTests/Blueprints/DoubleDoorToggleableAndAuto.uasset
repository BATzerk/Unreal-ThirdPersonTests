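; Double door that can be toggled on or off and opens automatically for Characters while on.
; SetIson stores the state, matches the door's open state to it and turns the light green for on, red for off.
; While on, entering BoxTrigger opens the door and leaving closes it.
; Entry uses the box's overlap event, but exit uses the actor-wide end overlap.
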(event OnComponentBeginOverlap(BoxTrigger)
  (params (OverlappedComponent :type Primitive%20Component%20Object%20Reference) (OtherActor :type Actor%20Object%20Reference) (OtherComp :type Primitive%20Component%20Object%20Reference) (OtherBodyIndex :type Integer) (bFromSweep :type Boolean) (SweepResult :type Hit%20Result%20Structure%20%28by%20ref%29))
  (Utilities|Casting|CastToCharacter OtherActor)
  (if (Variables|Default|GetIsOn)
    (CallFunction|SetIsOpen true)))

(event EventSetIson
  (params (Val :type Boolean))
  (bind _output_get (Variables|Default|SetIsOn Val))
  (CallFunction|SetIsOpen _output_get) ; When set IsOn, set IsOpen to the same.
  (if (Variables|Default|GetIsOn)
    (Rendering|Components|Light|SetLightColor "(R=0.137968,G=1.000000,B=0.135477,A=1.000000)" true)
    (else
      (Rendering|Components|Light|SetLightColor "(R=0.730000,G=0.081636,B=0.000000,A=1.000000)" true))))

(event Collision|EventActorEndOverlap
  (params (OtherActor :type Actor%20Object%20Reference))
  (Utilities|Casting|CastToCharacter OtherActor)
  (if (Variables|Default|GetIsOn)
    (CallFunction|SetIsOpen false)))

(fn ConstructionScript
  (|CallParentFunction))