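; Interactable in-world console that a character toggles engagement with, enabling keyboard input to navigate text menus on a screen widget.
; Menus live in a stack starting at the main menu; Up/Down move the current row and SpaceBar activates it.
; Each row's function string selects pushing the lights menu or popping back, and the current menu supplies the screen text.
; Setting lights volume is a print-only TODO stub.
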(event EventBeginPlay
  (CallFunction|PushMenu (Variables|Default|GetMenuMain)))

(event EventInteract
  (params (Character :type Character%20Object%20Reference))
  (bind _returnvalue (Game|GetPlayerController 0))
  (bind _asinteracty_character (Utilities|Casting|CastToInteractyCharacter Character))
  (Variables|Default|SetIsCharEngaged (not (Variables|Default|GetIsCharEngaged)))
  (Default|SetConsoleEngagement _asinteracty_character (Variables|Default|GetIsCharEngaged))
  ;[1 1 1] Enable/disable input based on engagement
  (if (Variables|Default|GetIsCharEngaged)
    (Input|EnableInput _returnvalue)
    (else
      (Input|DisableInput _returnvalue))))

(event Input|KeyboardEvents|Down
  (params (Key :type Key%20Structure :default "None"))
  (:Pressed
    (Default|ChangeCurrRow (Variables|Default|GetCurrMenu) 1)
    (CallFunction|RefreshScreenText)))

(event Input|KeyboardEvents|Up
  (params (Key :type Key%20Structure :default "None"))
  (:Pressed
    (Default|ChangeCurrRow (Variables|Default|GetCurrMenu) -1)
    (CallFunction|RefreshScreenText)))

(event Input|KeyboardEvents|SpaceBar
  (params (Key :type Key%20Structure :default "None"))
  (:Pressed
    (CallFunction|InteractCurrRow)
    (CallFunction|RefreshScreenText)))

(fn ConstructionScript)

(fn PushMenu
  (params (Menu :type Console%20Menu%20Object%20Reference))
  (Utilities|Array|Add (Variables|Default|GetCurrMenus) Menu)
  (CallFunction|UpdateCurrMenuRef)
  (CallFunction|RefreshScreenText))

(fn PopMenu
  (bind _currmenus (Variables|Default|GetCurrMenus))
  ;[1 1 1] If we have at least 2 menus (don't wanna pop Main menu)
  (if (>= (Utilities|Array|Length (Variables|Default|GetCurrMenus)) 2)
    ;[1 1 1] Remove currMenu
    (Utilities|Array|RemoveIndex _currmenus (Utilities|Array|LastIndex _currmenus))
    (CallFunction|UpdateCurrMenuRef)
    (CallFunction|RefreshScreenText)))

(fn SetScreenText
  (params (Str :type String))
  (bind _asconsole_screen_widget (Utilities|Casting|CastToConsoleScreenWidget (UserInterface|GetUserWidgetObject (Variables|Default|GetScreenWidget))))
  (Default|SetTextMain _asconsole_screen_widget Str))

(fn RefreshScreenText
  (bind _returntext (Default|GetScreenText (Variables|Default|GetCurrMenu)))
  (CallFunction|SetScreenText _returntext))

(fn UpdateCurrMenuRef
  (bind _currmenus (Variables|Default|GetCurrMenus))
  (Variables|Default|SetCurrMenu (Utilities|Array|Get(acopy) _currmenus (Utilities|Array|LastIndex _currmenus))))

(fn InteractCurrRow
  (bind _currrow (Default|GetCurrRow (Variables|Default|GetCurrMenu)))
  (bind _output_get (LocalVariables|SetCurrRow _currrow))
  (switch string (.interactfuncstr _output_get)
    (:Default
      (Development|PrintString "Oops! Console Menu InteractFuncStr not recognized:")
      (Development|PrintString (.interactfuncstr _output_get)))
    (:PopMenu
      (CallFunction|PopMenu))
    (:PushMenu_Lights
      (CallFunction|PushMenu (Variables|Default|GetMenuLights)))))

(fn SetLightsVolume
  (params (Volume :type Float%20%28single-precision%29))
  (Development|PrintString "Set lights! TODO: This.")
  (Development|PrintString (Utilities|String|ToString(Float) Volume)))