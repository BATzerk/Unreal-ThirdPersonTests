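; MovingABBox0 is a test interactable box that moves between positions PosA and PosB when switched on or off.
; The SetIsOn event plays the AnimateLoc timeline forward or in reverse, lerping BodyBox's relative location without sweep.
; BeginPlay sets the timeline play rate from its length divided by Duration, then calls SetIsOn(false).
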(event EventSetIson
  (params (Val :type Boolean))
  (if Val
    (bind _loc (Timeline|AnimateLoc Play)
      (:Update
        (Transformation|SetRelativeLocation (Variables|Default|GetBodyBox) (Math|Vector|Lerp(Vector) (Variables|Default|GetPosA) (Variables|Default|GetPosB) _loc) false false)))
    (else
      (Timeline|AnimateLoc Reverse))))

(event EventBeginPlay
  (|InitTimelineSpeed)
  (CallFunction|SetIson false))

(fn ConstructionScript)