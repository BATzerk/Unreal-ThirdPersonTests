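; ConsoleMenu is a text-based menu Blueprint that tracks a selected row and builds the menu as a single screen string.
; GetScreenText loops over the Rows array and appends each line from GetRowText, which prefixes the current row with a ">" cursor.
; ChangeCurrRow moves the selection by a delta clamped to the array bounds through SetCurrRow, and GetCurrRow returns the selected entry.
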(event EventBeginPlay)

(event EventTick
  (params (DeltaSeconds :type Float%20%28single-precision%29)))

(fn GetScreenText
  (for (_ _array_index) (Variables|Default|GetRows)
    (bind _returnstr (CallFunction|GetRowText _array_index))
    (LocalVariables|SetStr (Utilities|String|Append (LocalVariables|GetStr) " 
" _returnstr)))
  (return (LocalVariables|GetStr)))

(fn GetRowText
  (params (RowIndex :type Integer))
  (if (== RowIndex (Variables|Default|GetCurrRowIndex))
    (LocalVariables|SetPrefix "> ")
    (else
      (LocalVariables|SetPrefix "   ")))
  (return (Utilities|String|Append (LocalVariables|GetPrefix) (.rowstr (Utilities|Array|Get(acopy) (Variables|Default|GetRows) RowIndex)))))

(fn ChangeCurrRow
  (params (IndexDelta :type Integer))
  (bind _output_get (LocalVariables|SetNewIndex (+ IndexDelta (Variables|Default|GetCurrRowIndex))))
  (bind _output_get_2 (LocalVariables|SetNewIndex (Math|Integer|Clamp(Integer) _output_get 0 (- (Utilities|Array|Length (Variables|Default|GetRows)) 1))))
  (CallFunction|SetCurrRow _output_get_2))

(fn SetCurrRow
  (params (NewIndex :type Integer))
  (Variables|Default|SetCurrRowIndex NewIndex))

(fn GetCurrRow
  (return (Utilities|Array|Get(acopy) (Variables|Default|GetRows) (Variables|Default|GetCurrRowIndex))))